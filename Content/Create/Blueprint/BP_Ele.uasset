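; Elevator actor that moves its inside mesh vertically when its Box trigger is overlapped.
; Each overlap alternates via FlipFlop between playing and reversing the Ele timeline, which lerps the mesh's relative Z from zero to Higher.
; Begin and end overlap both call EvtCharView on the player's BP_ThirdPerson_Edit_ pawn for camera view changes, without checking the overlapping actor.
; The construction script sets the mesh's initial height from High.
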(event OnComponentBeginOverlap(Box)
  (params (OverlappedComponent :type Primitive%20Component%20Object%20Reference) (OtherActor :type Actor%20Object%20Reference) (OtherComp :type Primitive%20Component%20Object%20Reference) (OtherBodyIndex :type Integer) (bFromSweep :type Boolean) (SweepResult :type Hit%20Result%20Structure%20%28by%20ref%29))
  ;[0.349 0.8196 1] Event_Cam_Movements
  (bind _asbp_third_person_edit_ (Utilities|Casting|CastToBP_ThirdPerson_Edit_ (Game|Player|GetPlayerPawn 0)))
  (Default|EvtCharView _asbp_third_person_edit_)
  ;[1 1 1] Switch_
  (Utilities|FlowControl|FlipFlop
    (:A
      ;[0.9301 0.7454 0.3278] Elevator_Animation_
      (bind _newtrack_0 (Timeline|Ele Play)
        (:Update
          (Transformation|SetRelativeLocation (Variables|Default|GetSm_game_ElevatorInside) (Math|Vector|MakeVector 0.0 0.0 (Math|Float|Lerp 0.0 (Variables|Default|GetHigher) _newtrack_0)) false false))))
    (:B
      (Timeline|Ele Reverse))))

(event OnComponentEndOverlap(Box)
  (params (OverlappedComponent :type Primitive%20Component%20Object%20Reference) (OtherActor :type Actor%20Object%20Reference) (OtherComp :type Primitive%20Component%20Object%20Reference) (OtherBodyIndex :type Integer))
  ;[0.01033 0.4678 0.2623] Event_Cam_Cancel_
  (bind _asbp_third_person_edit_ (Utilities|Casting|CastToBP_ThirdPerson_Edit_ (Game|Player|GetPlayerPawn 0)))
  (Default|EvtCharView _asbp_third_person_edit_))

(fn ConstructionScript
  (Transformation|SetRelativeLocation (Variables|Default|GetSm_game_ElevatorInside) (Math|Vector|MakeVector 0.0 0.0 (Variables|Default|GetHigh)) false false))